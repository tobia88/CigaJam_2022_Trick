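; Loafer enemy character that patrols from an assigned patrol-point actor and can shoot and kill the player.
; The construction script snaps it to the first patrol point in world space, raised by its capsule half-height.
; Each tick, a line trace along its velocity updates IsFacingObstacle.
; AttackPlayer plays the shoot montage, while the separate DoPlayerDamage event kills the player outright through HandleDeath.
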(event `DoPlayerDamage`
  (bind _asbp_player_character (cast `/Game/ProjectTrick/Blueprints/Characters/Player/BP_PlayerCharacter` (`GameplayStatics.GetPlayerCharacter` 0)))
  (`/Game/ProjectTrick/Blueprints/Characters/Player/BP_PlayerCharacter.HandleDeath` _asbp_player_character))

(event `AttackPlayer`
  (`|PlayMontage` (`self.Mesh`) "/Game/ProjectTrick/Characters/Enemies/Loafer/Animations/AM_Enemy_Shoot.AM_Enemy_Shoot"))

(event `self.ReceiveTick`
  (params (DeltaSeconds :type "Float (single-precision)"))
  (bind _returnvalue (`self.K2_GetActorLocation`))
  (bind (_outhit _returnvalue_2) (`KismetSystemLibrary.LineTraceSingle` :`Start` _returnvalue :`End` (+ _returnvalue (* (`MovementComponent.Velocity` (`self.GetMovementComponent`)) 0.5)) :`TraceChannel` "TraceTypeQuery3" :`bTraceComplex` true :`DrawTime` 0.033333))
  (set `self.bIsFacingObstacle` _returnvalue_2))

(fn `UserConstructionScript`
  (bind _patrolpointactor (`self.PatrolPointActor`)
    (:`then`
      (bind _patrolpoints (`/Game/ProjectTrick/Blueprints/Actors/BP_PatrolPointsActor.PatrolPoints` _patrolpointactor))
      (if (> (`KismetArrayLibrary.Array_Length` _patrolpoints) 0)
        (bind (_returnvalue_x _returnvalue_y _returnvalue_z) (`KismetMathLibrary.BreakVector` (`KismetMathLibrary.TransformLocation` (`self.GetTransform` _patrolpointactor) (`|GetArrayItem` _patrolpoints))))
        (`self.K2_SetActorLocation` (`KismetMathLibrary.MakeVector` _returnvalue_x _returnvalue_y (+ _returnvalue_z (`CapsuleComponent.GetScaledCapsuleHalfHeight` (`self.CapsuleComponent`)))))))
    (:`else`)))