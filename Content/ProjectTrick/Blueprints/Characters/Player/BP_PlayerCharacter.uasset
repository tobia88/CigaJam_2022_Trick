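; Player character that moves relative to the camera, freezes its shadow actors on the controller's jump event, and handles death, restart and quit.
; Freezing flashes the screen through a timeline-weighted post-process material.
; Each tick re-gathers shadows, partially sorts them by distance (farthest last) and draws debug labels; RemoveAllShadows destroys only the first entry.
; Death plays a montage, then stops movement and calls the game mode's GameOver.
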(event `self.ReceiveBeginPlay`
  (bind _returnvalue (`KismetMaterialLibrary.CreateDynamicMaterialInstance` "/Game/ProjectTrick/Materials/MI_PP_FlashScreen.MI_PP_FlashScreen"))
  (set `self.PP_FlashScreen` _returnvalue)
  (bind _asbp_player_controller (cast `/Game/ProjectTrick/Blueprints/Core/BP_PlayerController` (`GameplayStatics.GetPlayerController` 0)))
  (add `/Game/ProjectTrick/Blueprints/Core/BP_PlayerController.HandleJumpEvent` _asbp_player_controller (delegate `SolidateShadow`)))

(event `SolidateShadow`
  (if (not (`self.bIsDead`))
    (bind _outactors (`GameplayStatics.GetAllActorsOfClass` "/Game/ProjectTrick/Blueprints/Actors/BP_PlayerShadowActor.BP_PlayerShadowActor_C"))
    (for _array_element _outactors
      (set `/Game/ProjectTrick/Blueprints/Actors/BP_PlayerShadowActor.bIsFreezed` true _array_element))
    ;[1 1 1] Flash Screen
    (if (> (`KismetArrayLibrary.Array_Length` _outactors) 0)
      (bind _outactors_2 (`GameplayStatics.GetAllActorsOfClass` "/Script/Engine.PostProcessVolume"))
      (for _array_element_2 _outactors_2
        (bind (_direction _flashscreenweight) (`Timeline|TL_FlashScreen` :!via `PlayFromStart`)
          (:`Update`
            (`PostProcessVolume.AddOrUpdateBlendable` _array_element_2 (`self.PP_FlashScreen`) _flashscreenweight)))))))

(event `self.ReceiveTick`
  (params (DeltaSeconds :type "Float (single-precision)"))
  (bind _transformcomponent (`PlayerCameraManager.TransformComponent` (`GameplayStatics.GetPlayerCameraManager` 0)))
  ;[1 1 1] Player Movement
  (`|ExecutionSequence`
    (:`then_0`
      (if (not (`self.bIsDead`))
        (`self.AddMovementInput` (+ (* (`self.GetInputAxisValue`) (`KismetMathLibrary.Vector_Normal2D` (`SceneComponent.GetForwardVector` _transformcomponent))) (* (`self.GetInputAxisValue`) (`KismetMathLibrary.Vector_Normal2D` (`SceneComponent.GetRightVector` _transformcomponent)))))))
    (:`then_1`
      (`self.SortShadowActorsByDistance`))))

(event `InputAction|Restart`
  (params (Key :type "Key Structure"))
  (:`Pressed`
    (bind _asbp_project_trick_game_mode (cast `/Game/ProjectTrick/Blueprints/Core/BP_ProjectTrickGameMode` (`GameplayStatics.GetGameMode`)))
    (`/Game/ProjectTrick/Blueprints/Core/BP_ProjectTrickGameMode.RestartGame` _asbp_project_trick_game_mode)))

(event `HandleDeath`
  (`|PlayMontage` (`self.Mesh`) "/Game/ProjectTrick/Characters/Player/Animations/AM_Player_Death.AM_Player_Death"
    (:`then`
      (set `self.bIsDead` true)
      (bind _asbp_project_trick_game_mode (cast `/Game/ProjectTrick/Blueprints/Core/BP_ProjectTrickGameMode` (`GameplayStatics.GetGameMode`)))
      (`/Game/ProjectTrick/Blueprints/Core/BP_ProjectTrickGameMode.GameOver` _asbp_project_trick_game_mode))))

(event `InputAction|RemoveAllShadows`
  (params (Key :type "Key Structure"))
  (bind _tmpshadowactors (`self.TmpShadowActors`))
  (:`Pressed`
    (if (> (`KismetArrayLibrary.Array_Length` _tmpshadowactors) 0)
      (`self.K2_DestroyActor` (`|GetArrayItem` _tmpshadowactors))
      (`KismetArrayLibrary.Array_Remove` _tmpshadowactors))))

(event `Key|Escape`
  (params (Key :type "Key Structure"))
  (:`Pressed`
    (`KismetSystemLibrary.QuitGame` null "Quit")))

(fn `SortShadowActorsByDistance`
  (bind _returnvalue (`self.K2_GetActorLocation`))
  (bind _outactors (`GameplayStatics.GetAllActorsOfClass` "/Game/ProjectTrick/Blueprints/Actors/BP_PlayerShadowActor.BP_PlayerShadowActor_C"))
  (bind _output_get (set `self.TmpShadowActors` _outactors))
  (for (_array_element _array_index) _output_get
    (bind _returnvalue_2 (- (`KismetArrayLibrary.Array_Length` _output_get) 1))
    (if (< _array_index _returnvalue_2)
      (if (> (`KismetMathLibrary.Vector_Distance2DSquared` (`self.K2_GetActorLocation` _array_element) _returnvalue) (`KismetMathLibrary.Vector_Distance2DSquared` _returnvalue (`self.K2_GetActorLocation` (`|GetArrayItem` _output_get _returnvalue_2))))
        (`KismetArrayLibrary.Array_Swap` (`self.TmpShadowActors`) _array_index _returnvalue_2))))
  ;[1 1 1] Debug
  (for (_array_element_2 _array_index_2) (`self.TmpShadowActors`)
    (`KismetSystemLibrary.DrawDebugString` (`self.K2_GetActorLocation` _array_element_2) (`KismetTextLibrary.Conv_TextToString` (`|FormatText` "Shadow::{index}::Distance::{distance}" _array_index_2 (`KismetMathLibrary.Vector_Distance2D` (`self.K2_GetActorLocation` _array_element_2) (`self.K2_GetActorLocation`)))) null (struct :`R` 1.0 :`G` 1.0 :`B` 1.0 :`A` 1.0) (`GameplayStatics.GetWorldDeltaSeconds`))))

(fn `UserConstructionScript`)