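; BP_PlayerShadowPoseActor is a visual stand-in that shows the player character's pose at the location of its owning shadow actor.
; On BeginPlay it copies the player's skeletal mesh into a PoseableMesh and stores dynamic material instances for every slot.
; Each tick it follows OwnerShadowActor and, unless that actor is frozen, copies the player's rotation and pose.
; A curve-driven mesh shake with debug capsule exists but is unconnected.
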(event `self.ReceiveBeginPlay`
  ;[1 1 1] Init Possable Mesh
  (`SkinnedMeshComponent.SetSkinnedAssetAndUpdate` (`self.PoseableMesh`) (`SkinnedMeshComponent.SkeletalMesh` (`Character.Mesh` (`GameplayStatics.GetPlayerCharacter` 0))) true)
  (for (_ _array_index) (`MeshComponent.GetMaterials` (`self.PoseableMesh`))
    (bind _returnvalue (`KismetMaterialLibrary.CreateDynamicMaterialInstance` "/Game/ProjectTrick/Materials/MI_PosableMesh.MI_PosableMesh"))
    (`PrimitiveComponent.SetMaterial` (`self.PoseableMesh`) _array_index _returnvalue)
    (`KismetArrayLibrary.Array_Add` (`self.PoseableMeshDynamicMats`) _returnvalue)))

(event `self.ReceiveTick`
  (params (DeltaSeconds :type "Float (single-precision)"))
  (bind _returnvalue (`GameplayStatics.GetPlayerCharacter` 0))
  (bind _ownershadowactor (`self.OwnerShadowActor`))
  (bind _poseablemesh (`self.PoseableMesh`))
  (`|ExecutionSequence`
    (:`then_0`
      (`/Engine/EditorBlueprintResources/StandardMacros.IsValid` _ownershadowactor
        (:`Is Valid`
          (`self.K2_SetActorLocation` (`self.K2_GetActorLocation` _ownershadowactor))
          ;[1 1 1] Pose Copy
          (if (not (`/Game/ProjectTrick/Blueprints/Actors/BP_PlayerShadowActor.bIsFreezed` (`self.OwnerShadowActor`)))
            (`/Engine/EditorBlueprintResources/StandardMacros.IsValid` _poseablemesh
              (:`Is Valid`
                (`self.K2_SetActorRotation` (`self.K2_GetActorRotation` _returnvalue))
                (`PoseableMeshComponent.CopyPoseFromSkeletalComponent` _poseablemesh (`Character.Mesh` _returnvalue))))))))))

(fn `UserConstructionScript`)