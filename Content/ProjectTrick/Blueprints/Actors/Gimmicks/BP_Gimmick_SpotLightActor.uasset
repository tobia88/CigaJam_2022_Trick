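; Spotlight gimmick that casts a player shadow actor while the player is inside its shadow trigger, with red, green or blue emissive material.
; Overlap stores the player and Tick spawns the shadow; leaving destroys it unless frozen.
; While activated, an optional timer clears the shadow and swings the light back and forth 90 degrees by timeline, disabling trigger collision mid-turn.
; Tick also drives emissive intensity from the activated state.
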(event `ClearPlayerShadowActor`
  (bind _playershadowinstance (`self.PlayerShadowInstance`)
    (:`then`
      (`self.K2_DestroyActor` _playershadowinstance))
    (:`else`)))

(event `self.ReceiveBeginPlay`
  (bind _rotateinterval (`self.RotateInterval`))
  (bind _skeletalmesh (`self.SkeletalMesh`))
  (`|ExecutionSequence`
    (:`then_0`
      (bind _output_get (set `self.FromRotation` (`self.K2_GetActorRotation`)))
      (set `self.ToRotation` (`KismetMathLibrary.MakeRotator` (.roll _output_get) (.pitch _output_get) (+ (.yaw _output_get) (`KismetMathLibrary.SelectFloat` 90.0 -90.0 (`self.RotateReverse`))))))
    (:`then_1`
      ;[1 1 1] Create Emissive Light Dynamic Material
      (bind _returnvalue (`KismetMaterialLibrary.CreateDynamicMaterialInstance` (`PrimitiveComponent.GetMaterial` _skeletalmesh 3)))
      (bind _output_get_2 (set `self.EmissiveLightDynamicMat` _returnvalue))
      (`PrimitiveComponent.SetMaterial` _skeletalmesh 3 _output_get_2))
    (:`then_2`
      ;[1 1 1] Rotation Timer
      (if (> _rotateinterval 0.0)
        (`KismetSystemLibrary.K2_SetTimerDelegate` (delegate `CustomEvent_0`) _rotateinterval true)))))

(event `CustomEvent_0`
  ;[1 1 1] Rotation Timer
  (if (`self.bIsActivated`)
    (`self.ClearPlayerShadowActor`)
    (`PrimitiveComponent.SetCollisionEnabled` (`self.BT_Shadow`) "NoCollision")
    (bind (_direction _rotatevalue) (`Timeline|TL_Rotate` :!via `PlayFromStart`)
      (:`Update`
        (`self.K2_SetActorRotation` (`KismetMathLibrary.RLerp` (`self.FromRotation`) (`self.ToRotation`) _rotatevalue true)))
      (:`Finished`
        (`|ExecutionSequence`
          (:`then_0`
            (bind _output_get (set `self.TmpRotation` (`self.FromRotation`)))
            (set `self.FromRotation` (`self.ToRotation`))
            (set `self.ToRotation` _output_get))
          (:`then_1`
            (`PrimitiveComponent.SetCollisionEnabled` (`self.BT_Shadow`) "QueryAndPhysics")))))))

(event `self.ReceiveTick`
  (params (DeltaSeconds :type "Float (single-precision)"))
  ;[1 1 1] Emissive Lighting Material Update
  (`MaterialInstanceDynamic.SetScalarParameterValue` (`self.EmissiveLightDynamicMat`) "EmissiveIntensity" (`KismetMathLibrary.SelectFloat` 5.0 0.0 (`self.bIsActivated`)))
  (bind _playercharacter (`self.PlayerCharacter`)
    (:`then`
      (`self.PlayerShadowInstance`
        (:`then`)
        (:`else`
          ;[1 1 1] Spawn Player Shadow
          (bind _returnvalue (`|SpawnActorFromClass` "/Game/ProjectTrick/Blueprints/Actors/BP_PlayerShadowActor.BP_PlayerShadowActor_C" (`self.GetTransform` _playercharacter) "Undefined" "OverrideRootScale" null self null))
          (set `self.PlayerShadowInstance` _returnvalue))))
    (:`else`)))

(event `self.BT_Shadow.OnComponentBeginOverlap`
  (params (OverlappedComponent :type "PrimitiveComponent Object Reference") (OtherActor :type "Actor Object Reference") (OtherComp :type "PrimitiveComponent Object Reference") (OtherBodyIndex :type Integer) (bFromSweep :type Boolean) (SweepResult :type "HitResult Structure (by ref)"))
  (bind _asbp_player_character (cast `/Game/ProjectTrick/Blueprints/Characters/Player/BP_PlayerCharacter` OtherActor))
  (`self.PlayerShadowInstance`
    (:`then`)
    (:`else`
      (set `self.PlayerCharacter` _asbp_player_character))))

(event `self.BT_Shadow.OnComponentEndOverlap`
  (params (OverlappedComponent :type "PrimitiveComponent Object Reference") (OtherActor :type "Actor Object Reference") (OtherComp :type "PrimitiveComponent Object Reference") (OtherBodyIndex :type Integer))
  (cast `/Game/ProjectTrick/Blueprints/Characters/Player/BP_PlayerCharacter` OtherActor)
  (set `self.PlayerCharacter` null)
  (bind _playershadowinstance (`self.PlayerShadowInstance`)
    (:`then`
      (if (not (`/Game/ProjectTrick/Blueprints/Actors/BP_PlayerShadowActor.bIsFreezed` _playershadowinstance))
        (`self.ClearPlayerShadowActor`)))
    (:`else`)))

(fn `UserConstructionScript`
  (`PrimitiveComponent.SetMaterialByName` (`self.SkeletalMesh`) "lambert5" (select `/Game/ProjectTrick/Misc/E_SensorColor` (`self.SensorColor`) :`NewEnumerator0` "/Game/ProjectTrick/Materials/MI_EmissiveLight_Red.MI_EmissiveLight_Red" :`NewEnumerator1` "/Game/ProjectTrick/Materials/MI_EmissiveLight_Green.MI_EmissiveLight_Green" :`NewEnumerator2` "/Game/ProjectTrick/Materials/MI_EmissiveLight_Blue.MI_EmissiveLight_Blue" :!type "MaterialInterface Object Reference")))