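; Light sensor gimmick actor that reacts to whether it is covered by shadow.
; The construction script picks a red, green or blue emissive material from SensorColor, which BeginPlay turns into a dynamic instance.
; Each tick it glows only while unshadowed, activates its OwningGimmickActor while shadowed, and sets every OwningLightActors entry to the inverse state.
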(event `self.ReceiveBeginPlay`
  (bind _skeletalmesh (`self.SkeletalMesh`))
  ;[1 1 1] Create Emissive Light Dynamic Material
  (bind _returnvalue (`KismetMaterialLibrary.CreateDynamicMaterialInstance` (`PrimitiveComponent.GetMaterial` _skeletalmesh 3)))
  (bind _output_get (set `self.EmissiveLightDynamicMat` _returnvalue))
  (`PrimitiveComponent.SetMaterial` _skeletalmesh 3 _output_get))

(event `self.ReceiveTick`
  (params (DeltaSeconds :type "Float (single-precision)"))
  (`|ExecutionSequence`
    (:`then_0`
      ;[1 1 1] Emissive Lighting Material Update
      (`MaterialInstanceDynamic.SetScalarParameterValue` (`self.EmissiveLightDynamicMat`) "EmissiveIntensity" (`KismetMathLibrary.SelectFloat` 5.0 0.0 (not (`self.bIsCoveredByShadow`)))))
    (:`then_1`
      (bind _owninggimmickactor (`self.OwningGimmickActor`)
        (:`then`
          (set `/Game/ProjectTrick/Blueprints/Actors/Gimmicks/BP_Gimmick_GateActor.bIsActivated` (`self.bIsCoveredByShadow`) _owninggimmickactor))
        (:`else`)))
    (:`then_2`
      (for _array_element (`self.OwningLightActors`)
        (set `/Game/ProjectTrick/Blueprints/Actors/Gimmicks/BP_Gimmick_SpotLightActor.bIsActivated` (not (`self.bIsCoveredByShadow`)) _array_element)))))

(fn `UserConstructionScript`
  (`PrimitiveComponent.SetMaterial` (`self.SkeletalMesh`) 3 (select `/Game/ProjectTrick/Misc/E_SensorColor` (`self.SensorColor`) :`NewEnumerator0` "/Game/ProjectTrick/Materials/MI_EmissiveLight_Red.MI_EmissiveLight_Red" :`NewEnumerator1` "/Game/ProjectTrick/Materials/MI_EmissiveLight_Green.MI_EmissiveLight_Green" :`NewEnumerator2` "/Game/ProjectTrick/Materials/MI_EmissiveLight_Blue.MI_EmissiveLight_Blue" :!type "MaterialInterface Object Reference")))