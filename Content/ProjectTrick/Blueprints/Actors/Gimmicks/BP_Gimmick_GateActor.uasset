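; Gate gimmick actor that blocks passage until activated, then hides its skeletal mesh and disables its collision.
; The construction script picks a red, green or blue emissive material from SensorColor, which BeginPlay wraps in a dynamic instance.
; Tick polls IsActivated to drive glow, collision and visibility.
; Tick also hides the front or back shadow blocker on the player's side, using a dot product with a small dead zone where both show.
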(event `self.ReceiveBeginPlay`
  (bind _skeletalmesh (`self.SkeletalMesh`))
  ;[1 1 1] Create Emissive Light Dynamic Material
  (bind _returnvalue (`KismetMaterialLibrary.CreateDynamicMaterialInstance` (`PrimitiveComponent.GetMaterial` _skeletalmesh 2)))
  (bind _output_get (set `self.EmissiveLightDynamicMat` _returnvalue))
  (`PrimitiveComponent.SetMaterial` _skeletalmesh 2 _output_get))

(event `self.ReceiveTick`
  (params (DeltaSeconds :type "Float (single-precision)"))
  (bind _returnvalue (`KismetMathLibrary.Dot_VectorVector` (`KismetMathLibrary.GetDirectionUnitVector` (`self.K2_GetActorLocation`) (`self.K2_GetActorLocation` (`GameplayStatics.GetPlayerCharacter` 0))) (`self.GetActorForwardVector`)))
  ;[1 1 1] Emissive Lighting Material Update
  (`MaterialInstanceDynamic.SetScalarParameterValue` (`self.EmissiveLightDynamicMat`) "EmissiveIntensity" (`KismetMathLibrary.SelectFloat` 5.0 0.0 (not (`self.bIsActivated`))))
  (`PrimitiveComponent.SetCollisionEnabled` (`self.SkeletalMesh`) (select `bool` (`self.bIsActivated`) :`false` "QueryAndPhysics" :`true` "NoCollision" :!type "ECollisionEnabled Enum"))
  (`SceneComponent.SetHiddenInGame` (`self.SkeletalMesh`) (`self.bIsActivated`) false)
  (`SceneComponent.SetHiddenInGame` (`self.ShadowBlocker_F`) (>= _returnvalue 0.1) false)
  (`SceneComponent.SetHiddenInGame` (`self.ShadowBlocker_B`) (<= _returnvalue -0.1) false))

(fn `UserConstructionScript`
  (`PrimitiveComponent.SetMaterial` (`self.SkeletalMesh`) 2 (select `/Game/ProjectTrick/Misc/E_SensorColor` (`self.SensorColor`) :`NewEnumerator0` "/Game/ProjectTrick/Materials/MI_EmissiveLight_Red.MI_EmissiveLight_Red" :`NewEnumerator1` "/Game/ProjectTrick/Materials/MI_EmissiveLight_Green.MI_EmissiveLight_Green" :`NewEnumerator2` "/Game/ProjectTrick/Materials/MI_EmissiveLight_Blue.MI_EmissiveLight_Blue" :!type "MaterialInterface Object Reference")))