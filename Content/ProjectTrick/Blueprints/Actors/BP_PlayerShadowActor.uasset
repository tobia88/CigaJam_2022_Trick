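; Player shadow actor that projects a 2D shadow aligned to an instigating light and, when frozen, becomes collidable.
; A scene capture renders only a spawned pose actor to a runtime render target, feeding a dynamic decal material.
; Each tick it follows the player's feet until frozen, updates opacity and collision, and line-traces to overlapped light sensors to flag shadow coverage.
; Debug box drawing is active, while lifetime and distance-based despawn logic is unconnected.
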(event `CustomEvent_0`
  (`self.K2_DestroyActor`))

(event `self.ReceiveBeginPlay`
  (bind _dm_box (`self.DM_Box`))
  (bind _sc_shadow_2d (`self.SC_Shadow_2D`))
  (`|ExecutionSequence`
    (:`then_0`
      ;[1 1 1] Spawn Shadow Pose Actor
      (bind _returnvalue (`|SpawnActorFromClass` "/Game/ProjectTrick/Blueprints/Actors/BP_PlayerShadowPoseActor.BP_PlayerShadowPoseActor_C" (`self.GetTransform`) "Undefined" "OverrideRootScale" null self null))
      (bind _output_get (set `self.ShadowPoseActor` _returnvalue))
      ;[1 1 1] Set RT
      (set `SceneCaptureComponent.ShowOnlyActors` (`|MakeArray` _output_get :!type "Actor Object Reference") _sc_shadow_2d)
      (bind _returnvalue_2 (`KismetRenderingLibrary.CreateRenderTarget2D` 256))
      (bind _output_get_2 (set `SceneCaptureComponent2D.TextureTarget` _returnvalue_2 _sc_shadow_2d))
      (set `self.TmpStoreShadowRT` _output_get_2))
    (:`then_2`
      ;[1 1 1] Create Decal DMI
      (bind _returnvalue_3 (`KismetMaterialLibrary.CreateDynamicMaterialInstance` (`PrimitiveComponent.GetMaterial` _dm_box 0)))
      (`PrimitiveComponent.SetMaterial` _dm_box 0 _returnvalue_3)
      (bind _output_get_3 (set `self.ShadowDecalDynamicMat` _returnvalue_3))
      (`MaterialInstanceDynamic.SetTextureParameterValue` _output_get_3 "Texture" (`self.TmpStoreShadowRT`)))))

(event `self.ReceiveTick`
  (params (DeltaSeconds :type "Float (single-precision)"))
  (bind _bc_shadowground (`self.BC_ShadowGround`))
  (bind _bc_shadowground_2 (`self.BC_ShadowGround`))
  (set `self.bIsInit` true)
  (`|ExecutionSequence`
    (:`then_0`
      ;[1 1 1] Update Collision bounds and position
      (if (not (`self.bIsFreezed`))
        (`self.UpdateCollisionBounds`)))
    (:`then_1`
      ;[1 1 1] Set Collision
      (`/Engine/EditorBlueprintResources/StandardMacros.IsValid` _bc_shadowground_2
        (:`Is Valid`
          (`PrimitiveComponent.SetCollisionEnabled` _bc_shadowground_2 (select `bool` (`self.bIsFreezed`) :`false` "NoCollision" :`true` "QueryAndPhysics" :!type "ECollisionEnabled Enum")))))
    (:`then_2`
      ;[1 1 1] Shadow Decal Color
      (`MaterialInstanceDynamic.SetVectorParameterValue` (`self.ShadowDecalDynamicMat`) "ShadowColor" (`KismetMathLibrary.SelectColor` (struct :`A` 0.5) (struct :`A` 1.0) (not (`self.bIsFreezed`)))))
    (:`then_3`
      ;[1 1 1] Debug
      (`/Engine/EditorBlueprintResources/StandardMacros.IsValid` _bc_shadowground
        (:`Is Valid`
          (`KismetSystemLibrary.DrawDebugBox` (`SceneComponent.K2_GetComponentLocation` _bc_shadowground) (`BoxComponent.GetScaledBoxExtent` _bc_shadowground) (`KismetMathLibrary.SelectColor` (struct :`R` 0.895833 :`G` 0.632615 :`B` 0.027888 :`A` 1.0) (struct :`R` 0.086709 :`G` 0.290413 :`B` 0.805555 :`A` 1.0) (`self.bIsFreezed`)) (`self.K2_GetActorRotation`) 0.033333 2.0))))
    (:`then_4`
      (bind _coveredlightcensoractor (`self.CoveredLightCensorActor`)
        (:`then`
          (bind (_outhit _returnvalue) (`KismetSystemLibrary.LineTraceSingleForObjects` (`SceneComponent.K2_GetComponentLocation` (`self.Capsule`)) (`self.K2_GetActorLocation` _coveredlightcensoractor) (`self.Object Types`) true (`|MakeArray` self (`GameplayStatics.GetPlayerCharacter` 0) (`self.InstigatorLight`) :!type "Actor Object Reference") "ForDuration" true (struct :`R` 1.0 :`A` 1.0) (struct :`G` 1.0 :`A` 1.0) 0.033333))
          (set `/Game/ProjectTrick/Blueprints/Actors/Gimmicks/BP_Gimmick_LightCensorActor.bIsCoveredByShadow` (and (== _coveredlightcensoractor (`.HitActor` (`GameplayStatics.BreakHitResult` _outhit))) _returnvalue) _coveredlightcensoractor))
        (:`else`)))))

(event `self.BC_Interaction.OnComponentBeginOverlap`
  (params (OverlappedComponent :type "PrimitiveComponent Object Reference") (OtherActor :type "Actor Object Reference") (OtherComp :type "PrimitiveComponent Object Reference") (OtherBodyIndex :type Integer) (bFromSweep :type Boolean) (SweepResult :type "HitResult Structure (by ref)"))
  (bind _asbp_light_censor_actor (cast `/Game/ProjectTrick/Blueprints/Actors/Gimmicks/BP_Gimmick_LightCensorActor` OtherActor))
  (set `self.CoveredLightCensorActor` _asbp_light_censor_actor))

(event `self.BC_Interaction.OnComponentEndOverlap`
  (params (OverlappedComponent :type "PrimitiveComponent Object Reference") (OtherActor :type "Actor Object Reference") (OtherComp :type "PrimitiveComponent Object Reference") (OtherBodyIndex :type Integer))
  (bind _asbp_light_censor_actor (cast `/Game/ProjectTrick/Blueprints/Actors/Gimmicks/BP_Gimmick_LightCensorActor` OtherActor))
  (set `/Game/ProjectTrick/Blueprints/Actors/Gimmicks/BP_Gimmick_LightCensorActor.bIsCoveredByShadow` false _asbp_light_censor_actor)
  (set `self.CoveredLightCensorActor` null)
  (`KismetSystemLibrary.PrintString` "Light Censor is out of covered"))

(event `self.ReceiveDestroyed`
  (bind _shadowposeactor (`self.ShadowPoseActor`)
    (:`then`
      (`self.K2_DestroyActor` _shadowposeactor))
    (:`else`)))

(fn `UpdateCollisionBounds`
  (bind _returnvalue (`GameplayStatics.GetPlayerCharacter` 0))
  (bind _instigatorlight (`self.InstigatorLight`))
  (bind (_returnvalue_roll _returnvalue_pitch _returnvalue_yaw) (`KismetMathLibrary.BreakRotator` (`self.K2_GetActorRotation` _instigatorlight)))
  (bind (_returnvalue_x _returnvalue_y _returnvalue_z) (`KismetMathLibrary.BreakVector` (`self.K2_GetActorLocation` _returnvalue)))
  (`/Engine/EditorBlueprintResources/StandardMacros.IsValid` _returnvalue
    (:`Is Valid`
      (`/Engine/EditorBlueprintResources/StandardMacros.IsValid` _instigatorlight
        (:`Is Valid`
          (`self.K2_SetActorTransform` (`KismetMathLibrary.MakeTransform` (`KismetMathLibrary.MakeVector` _returnvalue_x _returnvalue_y (- _returnvalue_z (`CapsuleComponent.GetScaledCapsuleHalfHeight` (`Character.CapsuleComponent` _returnvalue)))) (`KismetMathLibrary.MakeRotator` _returnvalue_roll _returnvalue_pitch (+ _returnvalue_yaw 90.0)) (`self.GetActorScale3D`))))))))

(fn `UserConstructionScript`
  (bind _dm_box (`self.DM_Box`))
  (bind _shadowlength (`self.ShadowLength`))
  (bind _sc_shadow_2d (`self.SC_Shadow_2D`))
  (bind _playerheight (`self.PlayerHeight`))
  (bind (_relativescale3d_x _relativescale3d_y _relativescale3d_z) (`KismetMathLibrary.BreakVector` (`SceneComponent.RelativeScale3D` _dm_box)))
  (`|ExecutionSequence`
    (:`then_0`
      ;[1 1 1] Shadow Decal
      (`SceneComponent.K2_SetRelativeTransform` _dm_box (`KismetMathLibrary.MakeTransform` (`KismetMathLibrary.MakeVector` _shadowlength (* _shadowlength -0.5) (* _relativescale3d_z -0.5)) (struct :`Yaw` 90.0) (`KismetMathLibrary.MakeVector` _shadowlength _shadowlength _relativescale3d_z)) false false))
    (:`then_1`
      ;[1 1 1] Set Shadow Camera
      (`SceneComponent.K2_SetRelativeLocation` _sc_shadow_2d (`KismetMathLibrary.MakeVector` -150.0 0.0 (* _playerheight 0.5)) false false)
      (set `SceneCaptureComponent2D.OrthoWidth` _playerheight _sc_shadow_2d))))